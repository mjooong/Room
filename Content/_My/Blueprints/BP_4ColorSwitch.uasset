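; BP_4ColorSwitch is an interactable switch that shows a question widget and checks the player's answer.
; Overlapping its Box reveals a text prompt and enables input, though leaving only hides the text without disabling input.
; Releasing F adds the pre-created WBP_SwitchUI with UI-only input and a mouse cursor.
; The widget's answer is compared to CurrentAnswer, firing right or wrong dispatchers; only wrong answers clear IsShowUI.
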(event OnComponentBeginOverlap(Box)
  (params (OverlappedComponent :type Primitive%20Component%20Object%20Reference) (OtherActor :type Actor%20Object%20Reference) (OtherComp :type Primitive%20Component%20Object%20Reference) (OtherBodyIndex :type Integer) (bFromSweep :type Boolean) (SweepResult :type Hit%20Result%20Structure%20%28by%20ref%29))
  ;[1 1 1] TextRender
  (Rendering|SetVisibility (Variables|Default|GetTextRender) true false)
  (Input|EnableInput (Game|GetPlayerController 0)))

(event OnComponentEndOverlap(Box)
  (params (OverlappedComponent :type Primitive%20Component%20Object%20Reference) (OtherActor :type Actor%20Object%20Reference) (OtherComp :type Primitive%20Component%20Object%20Reference) (OtherBodyIndex :type Integer))
  ;[1 1 1] TextRender
  (Rendering|SetVisibility (Variables|Default|GetTextRender) false false)
  (Input|EnableInput (Game|GetPlayerController 0)))

(event Custom|OnUserAnswer
  (params (UserInput :type Integer))
  (if (== UserInput (Variables|Default|GetCurrentAnswer))
    (Default|CallOnAnswerIsRight (Variables|Default|GetCurrentAnswer))
    (Development|PrintString "맞았다")
    (else
      (Default|CallOnAnswerIsWrong (Variables|Default|GetCurrentAnswer))
      (Development|PrintString "틀렸다")
      (Variables|Default|SetIsShowUI false))))

(event EventBeginPlay
  (Utilities|FlowControl|Sequence
    (:then_0
      (bind _returnvalue (UserInterface|CreateWidget "/Game/_My/Map/Level02/WBP_SwitchUI.WBP_SwitchUI_C"))
      (Variables|Default|SetSwitchUI _returnvalue))
    (:then_1
      (EventDispatchers|BindEventtoOnUserAnswer (Variables|Default|GetSwitchUI) (delegate Custom|OnUserAnswer)))))

(event Collision|EventActorBeginOverlap
  (params (OtherActor :type Actor%20Object%20Reference)))

(event EventTick
  (params (DeltaSeconds :type Float%20%28single-precision%29)))

(event Input|KeyboardEvents|F
  (params (Key :type Key%20Structure :default "None"))
  ;[1 1 1] "F" Open Viewport
  (:Released
    (if (not (Variables|Default|GetIsShowUI))
      (UserInterface|Viewport|AddtoViewport (Variables|Default|GetSwitchUI) 0)
      (Variables|Default|SetIsShowUI true)
      (Variables|/Script/Engine.PlayerController|SetbShowMouseCursor (Game|GetPlayerController 0) true)
      (Input|SetInputModeUIOnly (Game|GetPlayerController 0) 0 "DoNotLock"))))

(fn ConstructionScript)