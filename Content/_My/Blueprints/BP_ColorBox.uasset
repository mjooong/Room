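; BP_ColorBox is a colored, glowing cube that goes dark when hit, intended as a target for gunfire.
; The construction script creates a dynamic material on the Cube, and BeginPlay applies its configurable color and brightness.
; Any hit on the Cube zeroes the brightness, without checking what struck it, and fires the OnCubeHit dispatcher.
; ResetData relights it at a hardcoded brightness rather than the configured BrightnessOfLight.
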(event OnComponentHit(Cube)
  (params (HitComponent :type Primitive%20Component%20Object%20Reference) (OtherActor :type Actor%20Object%20Reference) (OtherComp :type Primitive%20Component%20Object%20Reference) (NormalImpulse :type Vector :default "0, 0, 0") (Hit :type Hit%20Result%20Structure%20%28by%20ref%29))
  (Rendering|Material|SetScalarParameterValue (Variables|Default|GetMaterialInstance) "빛의밝기" 0.0 :!class /Script/Engine.MaterialInstanceDynamic) ; 총에 맞으면 밝기 0
  (Default|CallOnCubeHit))

(event EventBeginPlay
  (Rendering|Material|SetVectorParameterValue (Variables|Default|GetMaterialInstance) "기본컬러" (Math|Conversions|ToLinearColor(Color) (Variables|Default|GetbasicColor)) :!class /Script/Engine.MaterialInstanceDynamic) ; 색상 변경
  (Rendering|Material|SetScalarParameterValue (Variables|Default|GetMaterialInstance) "빛의밝기" (Variables|Default|GetbrightnessOfLight) :!class /Script/Engine.MaterialInstanceDynamic) ; 빛의밝기 변경
)

(event Collision|EventActorBeginOverlap
  (params (OtherActor :type Actor%20Object%20Reference)))

(event EventTick
  (params (DeltaSeconds :type Float%20%28single-precision%29)))

(event Input|KeyboardEvents|G
  (params (Key :type Key%20Structure :default "None")))

(fn ConstructionScript
  (bind _returnvalue (Rendering|Material|CreateDynamicMaterialInstance (Variables|Default|GetCube) 0 0 "None" :!class /Script/Engine.PrimitiveComponent))
  (Variables|Default|SetMaterialInstance _returnvalue))

(fn ResetData
  (Rendering|Material|SetScalarParameterValue (Variables|Default|GetMaterialInstance) "빛의밝기" 5.0 :!class /Script/Engine.MaterialInstanceDynamic))