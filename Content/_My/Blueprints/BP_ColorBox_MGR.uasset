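; BP_ColorBox_MGR is a manager for a four-box hit-order puzzle that checks the sequence in which the ColorBoxes are struck.
; On BeginPlay it binds each box's OnCubeHit event, recording that box's ID into an input array.
; After four hits, it packs the IDs into a four-digit number and compares it to CorrectAnswer.
; It then fires a right or wrong dispatcher, resetting boxes and input when wrong.
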(event Custom|OnHitCube1
  (Development|PrintString "1번입니다")
  (CallFunction|AddUserInput 1))

(event Custom|OnHitCube4
  (Development|PrintString "4번입니다")
  (CallFunction|AddUserInput 4))

(event Custom|OnHitCube2
  (Development|PrintString "2번입니다")
  (CallFunction|AddUserInput 2))

(event Custom|OnHitCube3
  (Development|PrintString "3번입니다")
  (CallFunction|AddUserInput 3))

(event EventBeginPlay
  (EventDispatchers|BindEventtoOnCubeHit (Variables|ColorBox|GetColorBox1) (delegate Custom|OnHitCube1))
  (EventDispatchers|BindEventtoOnCubeHit (Variables|ColorBox|GetColorBox2) (delegate Custom|OnHitCube2))
  (EventDispatchers|BindEventtoOnCubeHit (Variables|ColorBox|GetColorBox3) (delegate Custom|OnHitCube3))
  (EventDispatchers|BindEventtoOnCubeHit (Variables|ColorBox|GetColorBox4) (delegate Custom|OnHitCube4)))

(event Collision|EventActorBeginOverlap
  (params (OtherActor :type Actor%20Object%20Reference)))

(event EventTick
  (params (DeltaSeconds :type Float%20%28single-precision%29)))

(fn ConstructionScript)

(fn AddUserInput
  (params (Cube_ID :type Integer))
  (Utilities|Array|SetArrayElem (Variables|Default|GetArrUserInput) (Variables|Default|GetnIndex) Cube_ID)
  (bind _output_get (Variables|Default|SetnIndex (+ (Variables|Default|GetnIndex) 1)))
  (if (== _output_get 4)
    (Development|PrintString "4번 맞음" true true "(R=1.000000,G=0.000000,B=0.000000,A=1.000000)")
    (bind _returnvalue (CallFunction|Make4Digit))
    (if (== _returnvalue (Variables|Default|GetCorrectAnswer))
      (Default|CallOnAnswerIsRight)
      (else
        (Default|CallOnAnswerIsrWrong)
        (Default|ResetData (Variables|ColorBox|GetColorBox1))
        (Default|ResetData (Variables|ColorBox|GetColorBox2))
        (Default|ResetData (Variables|ColorBox|GetColorBox3))
        (Default|ResetData (Variables|ColorBox|GetColorBox4))
        (Utilities|Array|SetArrayElem (Variables|Default|GetArrUserInput) 0 -1)
        (Utilities|Array|SetArrayElem (Variables|Default|GetArrUserInput) 1 -1)
        (Utilities|Array|SetArrayElem (Variables|Default|GetArrUserInput) 2 -1)
        (Utilities|Array|SetArrayElem (Variables|Default|GetArrUserInput) 3 -1)
        (Variables|Default|SetnIndex 0)))))

(fn Make4Digit
  (return (+ (* (Utilities|Array|Get(acopy) (Variables|Default|GetArrUserInput)) 1000) (* (Utilities|Array|Get(acopy) (Variables|Default|GetArrUserInput) 1) 100) (* (Utilities|Array|Get(acopy) (Variables|Default|GetArrUserInput) 2) 10) (Utilities|Array|Get(acopy) (Variables|Default|GetArrUserInput) 3))))